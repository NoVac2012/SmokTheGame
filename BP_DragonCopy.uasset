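; Player dragon character with Enhanced Input walking, looking, forward-only sprint, jumping and flight.
; A timed double-tap of jump launches into Flying mode, and a press after an arming delay drops to Falling, with cooldowns gating jumps.
; Movement follows control yaw, or full control rotation when flying.
; Tick enables controller-desired rotation while moving and, during ABP_Dragon turn-in-place, interpolates the actor toward the control yaw captured at turn start.
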(event Custom|OnTurnStart
  ;[1 0.007499 0.007499] TurnEvents
  (Variables|Camera|SetFollowCamDuringTurn false)
  (Variables|Camera|SetTurnStartControlYaw (.Yaw (Math|Rotator|BreakRotator (Pawn|GetControlRotation (Pawn|GetController) :!class /Script/Engine.Controller))))
  (Variables|Camera|SetFollowCamDuringTurn false)
  (Variables|/Game/Animations/ABP_Dragon.ABP_Dragon_C|SetCanTriggerTurn (Variables|StoreEssentialVariables|GetABP_Dragon) false))

(event Custom|OnTurnEnd
  ;[1 0.007499 0.007499] TurnEvents
  (Variables|Camera|SetFinishTurnAdjust true))

(event Custom|ActivateFly
  (bind _charactermovement (Variables|Character|GetCharacterMovement))
  (Pawn|Components|CharacterMovement|SetMovementMode (Variables|Character|GetCharacterMovement) "MOVE_Flying" 0)
  (Character|LaunchCharacter "0.000000,0.000000,1000.000000" false true)
  (Variables|/Script/Engine.CharacterMovementComponent|SetMaxFlySpeed _charactermovement 1.2e+03)
  (Variables|/Script/Engine.CharacterMovementComponent|SetBrakingDecelerationFlying _charactermovement 1e+03)
  (Variables|/Script/Engine.CharacterMovementComponent|SetMaxAcceleration _charactermovement 2048.0)
  (Variables|/Script/Engine.CharacterMovementComponent|SetbOrientRotationToMovement _charactermovement false)
  (Variables|Default|SetbUseControllerRotationYaw false)
  (Variables|Default|SetIsFlying true)
  (Variables|Default|SetExitArmTime (+ (Utilities|Time|GetGameTimeinSeconds) (Variables|Default|GetExitArmDelay)))
  (Variables|Default|SetTapCount 0))

(event Custom|DeactivateFly
  (if (Utilities|Enum|Equal(Enum) (Variables|/Script/Engine.CharacterMovementComponent|GetMovementMode (Variables|Character|GetCharacterMovement)) "MOVE_Flying")
    (Pawn|Components|CharacterMovement|SetMovementMode (Variables|Character|GetCharacterMovement) "MOVE_Falling" 0)
    (Variables|Default|SetIsFlying false)
    (Variables|Default|SetTapCount 0)
    (Variables|Jump|SetNextAllowedJumpTime (Math|Float|Max(Float) (Variables|Jump|GetNextAllowedJumpTime) (+ (Utilities|Time|GetGameTimeinSeconds) (Variables|Default|GetLandedLockOut))))))

(event Input|EnhancedActionEvents|EnhancedInputActionIA_DragonLook
  (params (ActionValue :type Vector%202D%20Structure) (ElapsedSeconds :type Float%20%28double-precision%29) (TriggeredSeconds :type Float%20%28double-precision%29) (InputAction :type Input%20Action%20Object%20Reference :default "/Game/Blueprints/Input/IA_DragonLook.IA_DragonLook"))
  ;[1 0.007499 0.007499] Look
  (Pawn|Input|AddControllerYawInput (.x ActionValue))
  (Pawn|Input|AddControllerPitchInput (.y ActionValue)))

(event Input|EnhancedActionEvents|EnhancedInputActionIA_DragonSprint
  (params (ActionValue :type Boolean) (ElapsedSeconds :type Float%20%28double-precision%29) (TriggeredSeconds :type Float%20%28double-precision%29) (InputAction :type Input%20Action%20Object%20Reference :default "/Game/Blueprints/Input/IA_DragonSprint.IA_DragonSprint"))
  ;[1 0.007499 0.007499] Sprint
  (:Triggered
    (if (> (Variables|Walking|GetAxisForward) 0.0)
      (Variables|/Script/Engine.CharacterMovementComponent|SetMaxWalkSpeed (Variables|Character|GetCharacterMovement) (Variables|Walking|GetSprint))
      (Variables|Walking|SetIsSprinting true)
      (else
        (Variables|/Script/Engine.CharacterMovementComponent|SetMaxWalkSpeed (Variables|Character|GetCharacterMovement) (Variables|Walking|GetWalkSpeed))
        (Variables|Walking|SetIsSprinting false))))
  (:Completed
    (Variables|/Script/Engine.CharacterMovementComponent|SetMaxWalkSpeed (Variables|Character|GetCharacterMovement) (Variables|Walking|GetWalkSpeed))
    (Variables|Walking|SetIsSprinting false)))

(event Input|EnhancedActionEvents|EnhancedInputActionIA_DragonJump
  (params (ActionValue :type Boolean) (ElapsedSeconds :type Float%20%28double-precision%29) (TriggeredSeconds :type Float%20%28double-precision%29) (InputAction :type Input%20Action%20Object%20Reference :default "/Game/Blueprints/Input/IA_DragonJump.IA_DragonJump"))
  (:Started
    (if (Variables|Default|GetIsFlying)
      (if (>= (Utilities|Time|GetGameTimeinSeconds) (Variables|Default|GetExitArmTime))
        (CallFunction|DeactivateFly)
        (Development|PrintString "deactivated"))
      (else
        (Utilities|FlowControl|Sequence
          (:then_0
            (if (> (Utilities|Time|GetGameTimeinSeconds) (Variables|Default|GetDoubleTapExpireTime))
              (Variables|Default|SetTapCount 0)))
          (:then_1
            (Variables|Default|SetTapCount (+ (Variables|Default|GetTapCount) 1))
            (Variables|Default|SetDoubleTapExpireTime (+ (Utilities|Time|GetGameTimeinSeconds) (Variables|Default|GetDoubleTapWindow)))
            (if (== (Variables|Default|GetTapCount) 2)
              (CallFunction|ActivateFly)
              (Development|PrintString "is flying")
              (elif (Math|Boolean|ANDBoolean (>= (Utilities|Time|GetGameTimeinSeconds) (Variables|Jump|GetNextAllowedJumpTime)) (Variables|Jump|GetJumpReady) (Utilities|Enum|Equal(Enum) (Variables|/Script/Engine.CharacterMovementComponent|GetMovementMode (Variables|Character|GetCharacterMovement)) "MOVE_Walking"))
                (Character|Jump)
                (Variables|Jump|SetNextAllowedJumpTime (+ (Utilities|Time|GetGameTimeinSeconds) (Variables|Jump|GetJumpCooldown)))))))))))

(event Input|EnhancedActionEvents|EnhancedInputActionIA_DragonMoveRL
  (params (ActionValue :type Float%20%28double-precision%29) (ElapsedSeconds :type Float%20%28double-precision%29) (TriggeredSeconds :type Float%20%28double-precision%29) (InputAction :type Input%20Action%20Object%20Reference :default "/Game/Blueprints/Input/IA_DragonMoveRL.IA_DragonMoveRL"))
  ;[1 0.007499 0.007499] Move
  (:Triggered
    (Variables|Walking|SetAxisRight ActionValue)
    (Pawn|Input|AddMovementInput (.Vector (CallFunction|RightDirectionCalculation)) ActionValue false))
  (:Completed
    (Variables|Walking|SetAxisRight 0.0)))

(event Input|EnhancedActionEvents|EnhancedInputActionIA_DragonMoveFB
  (params (ActionValue :type Float%20%28double-precision%29) (ElapsedSeconds :type Float%20%28double-precision%29) (TriggeredSeconds :type Float%20%28double-precision%29) (InputAction :type Input%20Action%20Object%20Reference :default "/Game/Blueprints/Input/IA_DragonMoveFB.IA_DragonMoveFB"))
  ;[1 0.007499 0.007499] Move
  (:Triggered
    (Variables|Walking|SetAxisForward ActionValue)
    (Pawn|Input|AddMovementInput (.ReturnValue (CallFunction|ForwardDirectionCalculation)) ActionValue false)
    (CallFunction|SprintActivation))
  (:Completed
    (CallFunction|SprintDeActivation)
    (Variables|Walking|SetAxisForward 0.0)))

(event EventBeginPlay
  ;[1 0.007499 0.007499] BeginPlay
  (CallFunction|AddMappingContext)
  (CallFunction|StoreCasttoAnimationBlueprint)
  (CallFunction|InitYawAccumulators)
  (Variables|Default|SetIsFlying false))

(event EventTick
  (params (DeltaSeconds :type Float%20%28single-precision%29))
  ;[1 0.007499 0.007499] Tick
  (if (Variables|Camera|GetYawIntDone)
    (bind _returnvalue (CallFunction|IsActorMoving))
    (CallFunction|SetActorandControlYaw DeltaSeconds _returnvalue)
    (else
      (CallFunction|InitYawAccumulators))))

(event EventOnLanded
  (params (Hit :type Hit%20Result%20Structure%20%28by%20ref%29))
  (Variables|Default|SetIsFlying false)
  (Variables|Jump|SetNextAllowedJumpTime (Math|Float|Max(Float) (Variables|Jump|GetNextAllowedJumpTime) (+ (Utilities|Time|GetGameTimeinSeconds) (Variables|Default|GetLandedLockOut))))
  (Variables|Default|SetTapCount 0))

(fn ConstructionScript)

(fn CanJumpCondition
  (return (Math|Boolean|ANDBoolean (>= (Utilities|Time|GetGameTimeinSeconds) (Variables|Jump|GetNextAllowedJumpTime)) (Character|CanJump) (not (AI|Components|NavMovement|IsFalling (Variables|Character|GetCharacterMovement))) (AI|Components|NavMovement|IsMovingonGround (Variables|Character|GetCharacterMovement)) (not (Variables|Default|GetIsFlying)))))

(fn RightDirectionCalculation
  (bind _returnvalue (Pawn|GetControlRotation :!class /Script/Engine.Pawn))
  (bind _charactermovement (Variables|Character|GetCharacterMovement))
  (bind _yaw (Math|Rotator|BreakRotator _returnvalue))
  (bind _movementmode (Variables|/Script/Engine.CharacterMovementComponent|GetMovementMode _charactermovement))
  (bind _returnvalue_2 (Math|Rotator|MakeRotator 0.0 0.0 _yaw))
  (bind _returnvalue_3 (Utilities|Select :Index _movementmode :MOVE_None _returnvalue_2 :MOVE_Walking _returnvalue_2 :MOVE_NavWalking "0, 0, 0" :MOVE_Falling _returnvalue_2 :MOVE_Swimming _returnvalue_2 :MOVE_Flying _returnvalue :MOVE_Custom _returnvalue_2))
  (return (Math|Vector|GetRightVector _returnvalue_3) _returnvalue_3))

(fn ForwardDirectionCalculation
  (bind _returnvalue (Pawn|GetControlRotation :!class /Script/Engine.Pawn))
  (bind _charactermovement (Variables|Character|GetCharacterMovement))
  (bind _yaw (Math|Rotator|BreakRotator _returnvalue))
  (bind _movementmode (Variables|/Script/Engine.CharacterMovementComponent|GetMovementMode _charactermovement))
  (bind _returnvalue_2 (Math|Rotator|MakeRotator 0.0 0.0 _yaw))
  (bind _returnvalue_3 (Utilities|Select :Index _movementmode :MOVE_None _returnvalue_2 :MOVE_Walking _returnvalue_2 :MOVE_NavWalking "0, 0, 0" :MOVE_Falling _returnvalue_2 :MOVE_Swimming _returnvalue_2 :MOVE_Flying _returnvalue :MOVE_Custom _returnvalue_2))
  (return (Math|Vector|GetForwardVector _returnvalue_3) _returnvalue_3))

(fn SprintActivation
  (if (and (<= (Variables|Walking|GetAxisForward) 0.1) (Variables|Walking|GetIsSprinting))
    (Variables|/Script/Engine.CharacterMovementComponent|SetMaxWalkSpeed (Variables|Character|GetCharacterMovement) (Variables|Walking|GetWalkSpeed))
    (Variables|Walking|SetIsSprinting false)))

(fn SprintDeActivation
  (Variables|Walking|SetAxisForward 0.0)
  (Variables|/Script/Engine.CharacterMovementComponent|SetMaxWalkSpeed (Variables|Character|GetCharacterMovement) (Variables|Walking|GetWalkSpeed))
  (Variables|Walking|SetIsSprinting false))

(fn SetActorandControlYaw
  (params (DeltaSec :type Float%20%28single-precision%29) (ShouldDriveControlYaw :type Boolean))
  (bind _returnvalue (Transformation|GetActorRotation))
  (bind _returnvalue_2 (Pawn|GetControlRotation :!class /Script/Engine.Pawn))
  (bind _turnstartcontrolyaw (Variables|Camera|GetTurnStartControlYaw))
  (bind _interpspeed (Variables|Camera|GetInterpSpeed))
  (bind _returnvalue_3 (Math|Rotator|MakeRotator 0.0 0.0 _turnstartcontrolyaw))
  (bind _yaw (Math|Rotator|BreakRotator _returnvalue_2))
  (bind _returnvalue_4 (Math|Interpolation|RInterpTo _returnvalue _returnvalue_3 DeltaSec _interpspeed))
  (bind _yaw_2 (Math|Rotator|BreakRotator _returnvalue_4))
  (Variables|Camera|SetShouldDriveControlYaw false)
  (if (== (Variables|/Game/Animations/ABP_Dragon.ABP_Dragon_C|GetIsTurningInPlace (Variables|StoreEssentialVariables|GetABP_Dragon)) true)
    (Transformation|SetActorRotation _returnvalue_4)
    (Variables|Camera|SetCurCtrlYaw _yaw_2)
    (Variables|Camera|SetActorYawAccum _yaw_2)
    (Variables|Camera|SetPrevActorYaw _yaw_2)
    (Variables|Camera|SetCurCtrlYaw _yaw)
    (Variables|Camera|SetPrevActorYaw _yaw)))

(fn InitYawAccumulators
  (Utilities|IsValid (Pawn|GetController)
    (:Is%20Valid
      (Variables|Camera|SetCurCtrlYaw (.Yaw (Math|Rotator|BreakRotator (Pawn|GetControlRotation (Pawn|GetController) :!class /Script/Engine.Controller))))
      (Variables|Camera|SetCurActorYaw (.Yaw (Math|Rotator|BreakRotator (Transformation|GetActorRotation))))
      (Variables|Camera|SetPrevControlYaw (Variables|Camera|GetCurCtrlYaw))
      (Variables|Camera|SetPrevActorYaw (Variables|Camera|GetCurActorYaw))
      (Variables|Camera|SetActorYawAccum (Variables|Camera|GetCurCtrlYaw))
      (Variables|Camera|SetActorYawAccum (Variables|Camera|GetCurActorYaw))
      (Variables|Camera|SetCtrlYawAccum (Variables|Camera|GetCurCtrlYaw))
      (Variables|Camera|SetYawIntDone true))))

(fn AddMappingContext
  (Input|AddMappingContext (PlayerController|LocalPlayerSubsystems|GetEnhancedInputLocalPlayerSubsystem (Game|GetPlayerController 0)) "/Game/Blueprints/Input/IMC_DragonMovement.IMC_DragonMovement" 0 "(bIgnoreAllPressedKeysUntilRelease=True,bForceImmediately=False,bNotifyUserSettings=False)"))

(fn StoreCasttoAnimationBlueprint
  (bind _asabp_dragon (Utilities|Casting|CastToABP_Dragon (Components|SkeletalMesh|GetAnimInstance (Variables|Character|GetMesh))))
  (Variables|StoreEssentialVariables|SetABP_Dragon _asabp_dragon))

(fn IsActorMoving
  (bind _returnvalue (Transformation|GetVelocity))
  (bind _movethreshold (Variables|Camera|GetMoveThreshold))
  (bind _charactermovement (Variables|Character|GetCharacterMovement))
  (bind _returnvalue_2 (Math|Vector|VectorLength _returnvalue))
  (bind _returnvalue_3 (AI|Components|NavMovement|IsFalling _charactermovement))
  (bind _returnvalue_4 (> _returnvalue_2 _movethreshold))
  (bind _returnvalue_5 (or _returnvalue_4 _returnvalue_3))
  (Variables|/Script/Engine.CharacterMovementComponent|SetbUseControllerDesiredRotation (Variables|Character|GetCharacterMovement) _returnvalue_5)
  (return (Math|Boolean|ORBoolean _returnvalue_5 _returnvalue_3 (Variables|Camera|GetFollowCamDuringTurn))))